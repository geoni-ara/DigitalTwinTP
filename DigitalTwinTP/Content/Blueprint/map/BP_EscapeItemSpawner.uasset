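; BP_EscapeItemSpawner scatters EscapeItem actors at random points inside its SpawnBox component.
; On BeginPlay it loops SpawnCount times, running a sphere overlap query of SpawnRadius against WorldDynamic objects, then spawning an item.
; The query result is unused, and the query and spawn each draw a separate random point, so overlaps do not affect placement.
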(event `self.ReceiveBeginPlay`
  (bind (_origin _boxextent) (`KismetSystemLibrary.GetComponentBounds` (`self.SpawnBox`)))
  (bind _returnvalue (`KismetMathLibrary.RandomPointInBoundingBox` _origin _boxextent))
  (for _ (range 1 (+ (`self.SpawnCount`) 1))
    (`KismetSystemLibrary.SphereOverlapActors` _returnvalue (`self.SpawnRadius`) (`|MakeArray` "ObjectTypeQuery2" :!type "EObjectTypeQuery Enum"))
    (`|SpawnActorFromClass` (`self.EscapeItem`) (`KismetMathLibrary.Conv_VectorToTransform` _returnvalue) "Undefined" "MultiplyWithRoot" null null)))

(fn `UserConstructionScript`)