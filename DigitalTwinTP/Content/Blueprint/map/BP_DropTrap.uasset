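; BP_DropTrap is a trap actor that drops its Cube when any actor overlaps the Box trigger.
; The overlap enables physics simulation on the Cube, then destroys the trap after a one-second delay.
; A second trigger, Box1, immediately stops an overlapping BP_Player's current movement and prints a stun message, with no lasting stun applied.
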(event `self.Box.OnComponentBeginOverlap`
  (params (OverlappedComponent :type "PrimitiveComponent Object Reference") (OtherActor :type "Actor Object Reference") (OtherComp :type "PrimitiveComponent Object Reference") (OtherBodyIndex :type Integer) (bFromSweep :type Boolean) (SweepResult :type "HitResult Structure (by ref)"))
  (if true
    (`PrimitiveComponent.SetSimulatePhysics` (`self.Cube`) true)
    (`KismetSystemLibrary.Delay` 1.0)
    (`self.K2_DestroyActor`)))

(event `self.ReceiveActorBeginOverlap`
  (params (OtherActor :type "Actor Object Reference")))

(event `self.Box1.OnComponentBeginOverlap`
  (params (OverlappedComponent :type "PrimitiveComponent Object Reference") (OtherActor :type "Actor Object Reference") (OtherComp :type "PrimitiveComponent Object Reference") (OtherBodyIndex :type Integer) (bFromSweep :type Boolean) (SweepResult :type "HitResult Structure (by ref)"))
  (bind _asbp_player (cast `/Game/Blueprint/BP_Player` OtherActor))
  (`MovementComponent.StopMovementImmediately` (`Character.CharacterMovement` _asbp_player))
  (`KismetSystemLibrary.PrintString` "기절"))

(fn `UserConstructionScript`)