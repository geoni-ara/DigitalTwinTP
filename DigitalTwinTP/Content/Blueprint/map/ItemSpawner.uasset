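; Item spawner actor that scatters random items from the ItemToSpawn list inside its SpawnBox volume on BeginPlay.
; For each of SpawnCount iterations it runs a sphere overlap at a random point in the box, then spawns an item.
; The overlap result does not gate spawning because the branch is always true, and the spawn location is a separate random roll from the tested point.
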(event `self.ReceiveBeginPlay`
  (bind (_origin _boxextent) (`KismetSystemLibrary.GetComponentBounds` (`self.SpawnBox`)))
  (bind _returnvalue (`KismetMathLibrary.RandomPointInBoundingBox` _origin _boxextent))
  (for _ (range 1 (+ (`self.SpawnCount `) 1))
    (`KismetSystemLibrary.SphereOverlapActors` _returnvalue (`self.SpawnRadius `) (`|MakeArray` "ObjectTypeQuery2" :!type "EObjectTypeQuery Enum"))
    (if true
      (`|SpawnActorFromClass` (`KismetArrayLibrary.Array_Random` (`self.ItemToSpawn`)) (`KismetMathLibrary.Conv_VectorToTransform` _returnvalue) "Undefined" "MultiplyWithRoot" null null))))

(fn `UserConstructionScript`)