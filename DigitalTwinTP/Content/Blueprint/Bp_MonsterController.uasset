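; Monster AI controller that chases the first player character and ends the game when it reaches them.
; Each Tick it line-traces from itself toward the player on the Camera channel and, on any blocking hit, issues an AI Move To, with success calling GameOver on BP_GameModeBase.
; A separate helper, not called in this graph, returns a monster speed scaled up linearly by Wariness.
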(event `self.ReceiveTick`
  (params (DeltaSeconds :type "Float (single-precision)"))
  (bind _returnvalue (`GameplayStatics.GetPlayerCharacter` 0))
  (bind _returnvalue_2 (`self.K2_GetActorLocation` _returnvalue))
  (bind (_outhit _returnvalue_3) (`KismetSystemLibrary.LineTraceSingle` (`self.K2_GetActorLocation`) _returnvalue_2 "TraceTypeQuery2"))
  (if _returnvalue_3
    (`|AIMoveTo` (`self.K2_GetPawn` self) _returnvalue_2 _returnvalue 100.0
      (:`OnSuccess`
        (bind _asbp_game_mode_base (cast `/Game/Blueprint/BP_GameModeBase` (`GameplayStatics.GetGameMode`)))
        (`/Game/Blueprint/BP_GameModeBase.GameOver` _asbp_game_mode_base)))))

(fn `setMonsterMaxSpeed`
  (params (MonsterSpeed :type "Float (double-precision)") (wariness :type Integer))
  (returns (result :type "Float (double-precision)"))
  (return (* MonsterSpeed (+ (* (`KismetMathLibrary.Conv_IntToDouble` wariness) 0.1) 1.0))))

(fn `UserConstructionScript`)